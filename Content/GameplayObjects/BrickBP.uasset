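; A breakable brick for a paddle-and-ball minigame that shows damage and dissolves away when destroyed.
; A dynamic material's DissolveAmount reflects health on damage; destruction disables collision and Tick advances the dissolve.
; When the dissolve completes, the brick decrements the game mode's remaining count and destroys itself; the last brick also triggers the controller's loading screen and removes the ball.
; Both hit events play a pitch-randomized click at the game instance's volume.
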(event `self.ReceiveBeginPlay`
  (bind _meshcomponent (`self.MeshComponent`))
  (bind _returnvalue (`PrimitiveComponent.CreateDynamicMaterialInstance` _meshcomponent 0 (`PrimitiveComponent.GetMaterial` _meshcomponent 0) "None"))
  (set `self.DissolveMaterial` _returnvalue))

(event `self.ReceiveTick`
  (params (DeltaSeconds :type "Float (single-precision)"))
  (if (`self.Destroyed?`)
    (bind _output_get (set `self.DissolveAmount` (+ (`self.DissolveAmount`) DeltaSeconds)))
    (if (>= _output_get 1.0)
      (bind _asminigames_game_mode_base (cast `MinigamesGameModeBase` (`GameplayStatics.GetGameMode`)))
      (bind _result (`/Engine/EditorBlueprintResources/StandardMacros.DecrementInt` (`MinigamesGameModeBase.RemainingBricks` _asminigames_game_mode_base))
        (:`  `
          (if (<= _result 0)
            (bind _asplayer_paddle_controller (cast `/Game/GameSystem/PlayerPaddleController` (`GameplayStatics.GetPlayerController` 0)))
            (`PaddleController.LoadingScreen` _asplayer_paddle_controller true)
            (bind _ball (`PaddleController.Ball` _asplayer_paddle_controller)
              (:`then`
                (`self.K2_DestroyActor` _ball))
              (:`else`
                _)))
          (`self.K2_DestroyActor`)))
      (else
        (`MaterialInstanceDynamic.SetScalarParameterValue` (`self.DissolveMaterial`) "DissolveAmount" (`self.DissolveAmount`))))))

(event `self.DestroyedBrick`
  (`self.SetActorEnableCollision` false)
  (set `self.Destroyed?` true)
  (bind _asminigame_instance_bp (cast `/Game/GameSystem/MinigameInstanceBP` (`GameplayStatics.GetGameInstance`)))
  (`GameplayStatics.PlaySound2D` "/Game/SFX/MA_SFX_Clicky_7_Edit.MA_SFX_Clicky_7_Edit" (`/Game/GameSystem/MinigameInstanceBP.GameVolume` _asminigame_instance_bp) (+ (* (- (`KismetMathLibrary.RandomFloat`) 0.5) 0.5) 1.0) 0.0 null null))

(event `self.DamagedBrick`
  (`MaterialInstanceDynamic.SetScalarParameterValue` (`self.DissolveMaterial`) "DissolveAmount" (/ (- 1.0 (`KismetMathLibrary.FClamp` (- (/ (`self.health`) (`self.maxhealth`)) 0.1) 0.0 0.5)) 2.0))
  (bind _asminigame_instance_bp (cast `/Game/GameSystem/MinigameInstanceBP` (`GameplayStatics.GetGameInstance`)))
  (`GameplayStatics.PlaySound2D` "/Game/SFX/MA_SFX_Clicky_7_Edit.MA_SFX_Clicky_7_Edit" (`/Game/GameSystem/MinigameInstanceBP.GameVolume` _asminigame_instance_bp) (+ (* (- (`KismetMathLibrary.RandomFloat`) 0.5) 0.5) 1.0) 0.0 null null))

(fn `UserConstructionScript`)